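; Top-down player character that moves on two input axes, snapping its Cube mesh to four facings and toggling pause with P.
; It shows a health widget, loses health and gets launched through ExperiencesDamage, and Tick respawns it at zero health.
; Capsule overlaps store the latest Checkpoint as the respawn point.
; The win trigger shows a win widget, then opens the main menu after a delay.
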(event `InputAxis|vertical`
  (params (AxisValue :type "Float (single-precision)"))
  ;[1 1 1] move speed
  (`self.AddMovementInput` (`KismetMathLibrary.MakeVector` (`self.Speed`)) AxisValue)
  (`self.TurnToDirection` (`KismetMathLibrary.MakeVector` AxisValue)))

(event `InputAxis|horizontal`
  (params (AxisValue :type "Float (single-precision)"))
  ;[1 1 1] move speed
  (`self.AddMovementInput` (`KismetMathLibrary.MakeVector` 0.0 (`self.Speed`)) AxisValue)
  (`self.TurnToDirection` (`KismetMathLibrary.MakeVector` 0.0 AxisValue)))

(event `self.ReceiveAnyDamage`
  (params (Damage :type "Float (single-precision)") (DamageType :type "DamageType Object Reference") (InstigatedBy :type "Controller Object Reference") (DamageCauser :type "Actor Object Reference"))
  ;[1 1 1] Health
)

(event `TurnToDirection`
  (params (direciton :type "Vector Structure"))
  (bind _cube (`self.Cube`))
  ;[1 1 1] turn fuctions
  (bind _output_get (set `self.Direciton` direciton))
  (bind _x (.x _output_get))
  (bind _y (.y _output_get))
  (if (> _x 0.0)
    (`SceneComponent.K2_SetRelativeRotation` _cube (`KismetMathLibrary.MakeRotator` 0.0) false false)
    (elif (< _x 0.0)
      (`SceneComponent.K2_SetRelativeRotation` _cube (`KismetMathLibrary.MakeRotator` 0.0 0.0 180.0) false false)
      (elif (> _y 0.0)
        (`SceneComponent.K2_SetRelativeRotation` _cube (`KismetMathLibrary.MakeRotator` 0.0 0.0 90.0) false false)
        (elif (< _y 0.0)
          (`SceneComponent.K2_SetRelativeRotation` _cube (`KismetMathLibrary.MakeRotator` 0.0 0.0 -90.0) false false))))))

(event `self.ReceiveBeginPlay`
  ;[1 1 1] Health
  (bind _returnvalue (`|CreateWidget` "/Game/Blueprints/health_widget.health_widget_C"))
  (`UserWidget.AddToViewport` _returnvalue 0))

(event `Key|P` :paused true
  (params (Key :type "Key Structure"))
  ;[1 1 1] pause function
  (:`Pressed`
    (if (`self.IsPaused`)
      (set `self.IsPaused` false)
      (`GameplayStatics.SetGamePaused` false)
      (else
        (set `self.IsPaused` true)
        (`GameplayStatics.SetGamePaused` true)))))

(event `self.CapsuleComponent.OnComponentBeginOverlap`
  (params (OverlappedComponent :type "PrimitiveComponent Object Reference") (OtherActor :type "Actor Object Reference") (OtherComp :type "PrimitiveComponent Object Reference") (OtherBodyIndex :type Integer) (bFromSweep :type Boolean) (SweepResult :type "HitResult Structure (by ref)"))
  ;[1 1 1] respawn functions
  (bind _ascheckpoint (cast `/Game/Blueprints/Checkpoint` OtherActor))
  (set `self.SpawnPoint` _ascheckpoint))

(event `Respawn`
  ;[1 1 1] respawn functions
  (`self.K2_SetActorLocation` (`self.K2_GetActorLocation` (`self.SpawnPoint`))))

(event `Experiences Damage`
  (params (NewParam :type "Vector Structure"))
  ;[1 1 1] damage health
  (`self.LaunchCharacter` (* NewParam (600.0 600.0 600.0)))
  (set `self.health` (- (`self.health`) 5.0)))

(event `self.ReceiveTick`
  (params (DeltaSeconds :type "Float (single-precision)"))
  ;[1 1 1] damage health
  (if (<= (`self.health`) 0.0)
    (`self.Respawn`)
    (set `self.health` 100.0)))

(event `self.Wintriggger.OnActorBeginOverlap`
  (params (OverlappedActor :type "Actor Object Reference") (OtherActor :type "Actor Object Reference"))
  ;[1 1 1] win screen
  (`KismetSystemLibrary.PrintString` "win")
  (bind _returnvalue (`|CreateWidget` "/Game/UI/winSreen_widget.winSreen_widget_C"))
  (`UserWidget.AddToViewport` _returnvalue 0)
  (`KismetSystemLibrary.Delay` 3.5)
  (`GameplayStatics.OpenLevelBySoftObjectPtr` "/Game/Main_Menu_Map.Main_Menu_Map"))

(fn `PBAFUN`
  (if (`self.PBABool`)
    (`KismetSystemLibrary.PrintString` "True")
    (else
      (`KismetSystemLibrary.PrintString` "False"))))

(fn `UserConstructionScript`)