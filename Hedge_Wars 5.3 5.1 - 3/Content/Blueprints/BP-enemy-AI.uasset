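; Enemy character Blueprint that chases pawns it sees and hurts the top-down player on contact.
; Pawn sensing sets a sensing flag and issues an AI MoveTo toward the seen pawn.
; A capsule hit on the player character calls its damage handler with the enemy's forward vector, then halts movement and briefly sets a stunned flag.
; The stunned flag is never read here, and separate ApplyDamage and CanAttack-reset nodes are unconnected.
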(event `self.PawnSensing.OnSeePawn`
  (params (Pawn :type "Pawn Object Reference"))
  (set `self.sensing Player` true)
  (`self.followPlayer`))

(event `followPlayer`
  (set `self.can attack` true)
  (if (`self.sensing Player`)
    (`|AIMoveTo` self (0.0 0.0 0.0) (stale `self.PawnSensing.OnSeePawn` Pawn))))

(event `self.CapsuleComponent.OnComponentHit`
  (params (HitComponent :type "PrimitiveComponent Object Reference") (OtherActor :type "Actor Object Reference") (OtherComp :type "PrimitiveComponent Object Reference") (NormalImpulse :type "Vector Structure") (Hit :type "HitResult Structure (by ref)"))
  (bind _astop__down__character (cast `/Game/Blueprints/Top-Down-Character` OtherActor))
  (`/Game/Blueprints/Top-Down-Character.Experiences Damage` _astop__down__character (`self.GetActorForwardVector`))
  (`self.Cooldown`))

(event `Cooldown`
  (set `self.Enemy Stunned` true)
  (`MovementComponent.StopMovementImmediately` (`self.CharacterMovement`))
  (`KismetSystemLibrary.Delay` 1.0)
  (set `self.Enemy Stunned` false))

(fn `UserConstructionScript`)