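; A size power-up pickup actor that enlarges the top-down player character.
; When a Top-Down-Character overlaps its Box, it runs PowerUp on that character and then destroys itself.
; PowerUp multiplies the character's current scale by IncreaseSize and sets its Camera to a fixed relative location, with no timer or revert logic.
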(event `self.Box.OnComponentBeginOverlap`
  (params (OverlappedComponent :type "PrimitiveComponent Object Reference") (OtherActor :type "Actor Object Reference") (OtherComp :type "PrimitiveComponent Object Reference") (OtherBodyIndex :type Integer) (bFromSweep :type Boolean) (SweepResult :type "HitResult Structure (by ref)"))
  (bind _astop__down__character (cast `/Game/Blueprints/Top-Down-Character` OtherActor))
  (`self.Power Up` _astop__down__character)
  (`self.K2_DestroyActor`))

(event `Power Up`
  (params (Character :type "/Game/Blueprints/Top-Down-Character Object Reference"))
  (bind (_returnvalue_x _returnvalue_y _returnvalue_z) (`KismetMathLibrary.BreakVector` (`self.GetActorScale3D` Character)))
  (bind _increasesize (`self.IncreaseSize`))
  (`self.SetActorScale3D` Character (`KismetMathLibrary.MakeVector` (* _returnvalue_x _increasesize) (* _returnvalue_y _increasesize) (* _returnvalue_z _increasesize)))
  (`SceneComponent.K2_SetRelativeLocation` (`/Game/Blueprints/Top-Down-Character.Camera` Character) (-18.0 50.0 1500.0) false false))

(fn `UserConstructionScript`)